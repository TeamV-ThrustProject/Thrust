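; Player Controller component that drives a scan effect centered on the controlled pawn, faded in and out through StartScan and EndScan.
; A state machine advances normalized scan time, publishes it to MPC_Scan with pawn location, and stops ticking when faded out.
; A lazily spawned BP_ScanActor supplies the post-process material, weighted by an optional curve, and grid-snapped Niagara.
; On fade-out it hides the Niagara and optionally destroys the actor.
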(event EventBeginPlay
  (bind _as플레이어_컨트롤러 (Utilities|Casting|CastToPlayerController (Components|GetOwner))
    (:then
      (Variables|Setting|SetPlayerController _as플레이어_컨트롤러)
      (Scan|State디폴트|UpdateScanState "NewEnumerator2" true)
      (Rendering|Material|SetScalarParameterValue "/Game/TESTING/MPC_Scan.MPC_Scan" "GridCellSize" (Variables|Default|GetGridCellSize) :!class /Script/Engine.KismetMaterialLibrary)
      (Rendering|Material|SetScalarParameterValue "/Game/TESTING/MPC_Scan.MPC_Scan" "Range" (Variables|Default|GetRange) :!class /Script/Engine.KismetMaterialLibrary))
    (:CastFailed
      (Scan|State디폴트|UpdateScanState "NewEnumerator4" true))))

(event EventTick
  (params (DeltaSeconds :type Float%20%28single-precision%29))
  (Scan|UpdateScanTime DeltaSeconds)
  (switch Utilities|FlowControl|Switch|SwitchonEBP_Scan_State (Scan|State디폴트|GetScanState)
    (:NewEnumerator0
      (Scan|Actor|UpdateScanPPBlendWeight :!label _label))
    (:NewEnumerator1
      _)
    (:NewEnumerator2
      (goto _label))
    (:NewEnumerator3
      _))
  (Scan|UpdateScanLocation))

(fn StartScan
  (switch Utilities|FlowControl|Switch|SwitchonEBP_Scan_State (Scan|State디폴트|GetScanState)
    (:NewEnumerator2
      _)
    (:NewEnumerator3
      _))
  (Scan|State디폴트|UpdateScanState "NewEnumerator0" false))

(fn EndScan
  (switch Utilities|FlowControl|Switch|SwitchonEBP_Scan_State (Scan|State디폴트|GetScanState)
    (:NewEnumerator0
      _)
    (:NewEnumerator1
      _))
  (Scan|State디폴트|UpdateScanState "NewEnumerator2" false))

(fn GetScanState
  (return (Variables|Scan|State디폴트|GetState)))

(fn UpdateScanState
  (params (State :type EBP_Scan_State%20Enum :default "NewEnumerator0") (bForce :type Boolean))
  (bind _scan_actor (Variables|Scan|Actor|GetScan%20Actor))
  (bind _scan_actor_2 (Variables|Scan|Actor|GetScan%20Actor))
  (bind _niagara (Variables|/Game/TESTING/BP_ScanActor.BP_ScanActor_C|GetNiagara _scan_actor))
  (bind _niagara_2 (Variables|/Game/TESTING/BP_ScanActor.BP_ScanActor_C|GetNiagara _scan_actor_2))
  (if (or (Utilities|Enum|NotEqual(Enum) State (Variables|Scan|State디폴트|GetState)) bForce)
    (Utilities|FlowControl|Sequence
      (:then_0
        ;[1 1 1] EXIT CURRENT STATE
        (switch Utilities|FlowControl|Switch|SwitchonEBP_Scan_State (Variables|Scan|State디폴트|GetState)
          (:NewEnumerator1
            (Rendering|Material|SetScalarParameterValue "/Game/TESTING/MPC_Scan.MPC_Scan" "bFadein" 0.0 :!class /Script/Engine.KismetMaterialLibrary))
          (:NewEnumerator3
            (Rendering|Material|SetScalarParameterValue "/Game/TESTING/MPC_Scan.MPC_Scan" "bFadeout" 0.0 :!class /Script/Engine.KismetMaterialLibrary)
            (Components|Tick|SetComponentTickEnabled true)
            (Utilities|IsValid _scan_actor_2
              (:Is%20Valid
                (Utilities|IsValid _niagara_2
                  (:Is%20Valid
                    (Rendering|SetVisibility _niagara_2 true false))))))))
      (:then_1
        ;[1 1 1] ENTER NEW STATE
        (bind _output_get (Variables|Scan|State디폴트|SetState State))
        (switch Utilities|FlowControl|Switch|SwitchonEBP_Scan_State _output_get
          (:NewEnumerator1
            (Rendering|Material|SetScalarParameterValue "/Game/TESTING/MPC_Scan.MPC_Scan" "bFadein" 1.0 :!class /Script/Engine.KismetMaterialLibrary)
            (Scan|Actor|UpdateScanPPBlendWeight))
          (:NewEnumerator3
            (Rendering|Material|SetScalarParameterValue "/Game/TESTING/MPC_Scan.MPC_Scan" "bFadeout" 1.0 :!class /Script/Engine.KismetMaterialLibrary)
            (Scan|Actor|UpdateScanPPBlendWeight)
            (Utilities|FlowControl|Sequence
              (:then_0
                (Utilities|IsValid _scan_actor
                  (:Is%20Valid
                    (Utilities|IsValid _niagara
                      (:Is%20Valid
                        (Rendering|SetVisibility _niagara false false))))))
              (:then_1
                (Components|Tick|SetComponentTickEnabled false :!label _label)
                (Scan|Actor|DestroyPPA))))
          (:NewEnumerator4
            (goto _label))))
      (:then_2
        (return true)))
    (else
      (return false))))

(fn UpdateScanTime
  (params (DeltaTime :type Float%20%28double-precision%29))
  (Utilities|FlowControl|Sequence
    (:then_0
      (switch Utilities|FlowControl|Switch|SwitchonEBP_Scan_State (Scan|State디폴트|GetScanState)
        (:NewEnumerator0
          (bind _output_get (Variables|Scan|Material|SetScanNomalizeTime (+ (Variables|Scan|Material|GetScanNomalizeTime) (* DeltaTime (Variables|Setting|Speed|GetFadeInSpeed)))))
          (if (>= _output_get 1.0)
            (Variables|Scan|Material|SetScanNomalizeTime 1.0)
            (Scan|State디폴트|UpdateScanState "NewEnumerator1" false)))
        (:NewEnumerator2
          (bind _output_get_2 (Variables|Scan|Material|SetScanNomalizeTime (- (Variables|Scan|Material|GetScanNomalizeTime) (* DeltaTime (Variables|Setting|Speed|GetFadeOutSpeed)))))
          (if (<= _output_get_2 0.0)
            (Variables|Scan|Material|SetScanNomalizeTime 0.0)
            (Scan|State디폴트|UpdateScanState "NewEnumerator3" false)))
        (:NewEnumerator4
          (return false)))
      (Rendering|Material|SetScalarParameterValue "/Game/TESTING/MPC_Scan.MPC_Scan" "NomalizedTime" (Variables|Scan|Material|GetScanNomalizeTime) :!class /Script/Engine.KismetMaterialLibrary))
    (:then_1
      (return true))))

(fn GetScanPPActor
  (bind _ppmaterial (Variables|Setting|Material|GetPPMaterial))
  (Utilities|IsValid (Variables|Scan|Actor|GetScan%20Actor)
    (:Is%20Valid
      (return (Variables|Scan|Actor|GetScan%20Actor)))
    (:Is%20Not%20Valid
      (bind _returnvalue (Game|SpawnActorfromClass "/Game/TESTING/BP_ScanActor.BP_ScanActor_C" (Math|Transform|MakeTransform "0, 0, 0") "Undefined" "MultiplyWithRoot" 0 0))
      (Variables|Scan|Actor|SetScan%20Actor _returnvalue)
      (Utilities|FlowControl|Sequence
        (:then_0
          (Utilities|IsValid (Variables|Scan|Material|GetPPMID)
            (:Is%20Valid
              _)
            (:Is%20Not%20Valid
              (Utilities|IsValid _ppmaterial
                (:Is%20Valid
                  (bind _returnvalue_2 (Rendering|Material|CreateDynamicMaterialInstance _ppmaterial "None" "None" :!class /Script/Engine.KismetMaterialLibrary))
                  (bind _output_get (Variables|Scan|Material|SetPPMID _returnvalue_2))))))
          (Utilities|IsValid (Variables|/Game/TESTING/BP_ScanActor.BP_ScanActor_C|GetPostProcess (Variables|Scan|Actor|GetScan%20Actor))
            (:Is%20Valid
              (Utilities|Struct|SetmembersinPostProcessSettings (Variables|/Script/Engine.PostProcessComponent|GetSettings (Variables|/Game/TESTING/BP_ScanActor.BP_ScanActor_C|GetPostProcess (Variables|Scan|Actor|GetScan%20Actor))) (Utilities|Struct|MakeWeightedBlendables (Utilities|Array|MakeArray (Utilities|Struct|MakeWeightedBlendable 1.0 (Variables|Scan|Material|GetPPMID))))))))
        (:then_1
          (return (Variables|Scan|Actor|GetScan%20Actor)))))))

(fn DestroyPPA
  (if (and (Utilities|IsValid (Variables|Scan|Actor|GetScan%20Actor)) (Variables|Setting|GetbDestroyActor))
    (Actor|DestroyActor (Variables|Scan|Actor|GetScan%20Actor))
    (Variables|Scan|Actor|SetScan%20Actor 0)))

(fn UpdateScanPPBlendWeight
  (bind _blendcurve (Variables|Setting|Material|GetBlendCurve))
  (bind _scannomalizetime (Variables|Scan|Material|GetScanNomalizeTime))
  (Utilities|IsValid _blendcurve
    (:Is%20Valid
      (LocalVariables|SetThisTime (Math|Curves|GetFloatValue _blendcurve _scannomalizetime)))
    (:Is%20Not%20Valid
      (LocalVariables|SetThisTime _scannomalizetime)))
  (bind _newparam (Scan|Actor|GetScanPPActor))
  (Utilities|IsValid _newparam
    (:Is%20Valid
      (Utilities|IsValid (Variables|/Game/TESTING/BP_ScanActor.BP_ScanActor_C|GetPostProcess _newparam)
        (:Is%20Valid
          (Variables|/Script/Engine.PostProcessComponent|SetBlendWeight (Variables|/Game/TESTING/BP_ScanActor.BP_ScanActor_C|GetPostProcess _newparam) (LocalVariables|GetThisTime)))))))

(fn UpdateScanLocation
  (bind _scan_actor (Variables|Scan|Actor|GetScan%20Actor))
  (bind _playercontroller (Variables|Setting|GetPlayerController))
  (bind _returnvalue (Pawn|GetControlledPawn _playercontroller))
  (bind _niagara (Variables|/Game/TESTING/BP_ScanActor.BP_ScanActor_C|GetNiagara _scan_actor))
  (Utilities|IsValid _playercontroller
    (:Is%20Valid
      (Utilities|IsValid _returnvalue
        (:Is%20Valid
          (bind _output_get (LocalVariables|SetNewLocalVar (Transformation|GetActorLocation _returnvalue)))
          (Rendering|Material|SetVectorParameterValue "/Game/TESTING/MPC_Scan.MPC_Scan" "Location" (Math|Conversions|ToLinearColor(Vector) _output_get) :!class /Script/Engine.KismetMaterialLibrary)
          (Utilities|IsValid _scan_actor
            (:Is%20Valid
              (Utilities|IsValid _niagara
                (:Is%20Valid
                  (Transformation|SetWorldLocation _niagara (Class|KismetMathLibrary|VectorSnappedtoGrid (LocalVariables|GetNewLocalVar) (Variables|Default|GetGridCellSize)) false true))))))))))